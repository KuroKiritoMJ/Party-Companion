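; HUD actor for a topic-based card game that shows the PickTopic widget on BeginPlay and picks three topics.
; GenerateTopicSelection re-rolls indices from 1 to 17 to avoid repeats, filling Topic1–3 from TopicsArray.
; GetCardInTopic re-rolls against CardsPlayed, but its check, record and returned card each use separate random calls.
; The A key is a debug draw for topic 1, though IDintoTopic's ID-to-topic switch is unconnected.
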(event Custom|PickCards_Event
  (bind _topics_presented (CallFunction|GenerateTopicSelection))
  (Variables|Default|SetTopic1 (Utilities|Array|Get(acopy) (Variables|Default|GetTopics_Array) (Utilities|Array|Get(acopy) _topics_presented)))
  (Variables|Default|SetTopic2 (Utilities|Array|Get(acopy) (Variables|Default|GetTopics_Array) (Utilities|Array|Get(acopy) _topics_presented 1)))
  (Variables|Default|SetTopic3 (Utilities|Array|Get(acopy) (Variables|Default|GetTopics_Array) (Utilities|Array|Get(acopy) _topics_presented 2))))

(event EventBeginPlay
  (bind _returnvalue (UserInterface|CreateWidget "/Game/Blueprints/PickTopic.PickTopic_C"))
  (UserInterface|Viewport|AddtoViewport _returnvalue 0)
  (CallFunction|PickCardsEvent))

(event Collision|EventActorBeginOverlap
  (params (OtherActor :type Actor%20Object%20Reference)))

(event EventTick
  (params (DeltaSeconds :type Float%20%28single-precision%29)))

(event Input|KeyboardEvents|A
  (params (Key :type Key%20Structure :default "None"))
  (:Pressed
    (bind _newparam1 (CallFunction|IDintoTopic 1))
    (CallFunction|GetCardinTopic _newparam1 1)
    (Development|PrintString "Hello")))

(fn ConstructionScript)

(fn GenerateTopicSelection
  (for _index (range 0 2)
    (switch int _index
      (:0
        (bind _output_get (Variables|Default|SetGenerate_Var (Math|Random|RandomIntegerinRange 1 17)))
        (bind _output_get_2 (Variables|Default|SetGenerate_NoRepeat_1 _output_get))
        (Utilities|Array|Add (Variables|Default|GetGenerate_Return) _output_get_2))
      (:1
        (bind _output_get_3 (Variables|Default|SetGenerate_Var (Math|Random|RandomIntegerinRange 1 17) :!label _label))
        (if (!= _output_get_3 (Variables|Default|GetGenerate_NoRepeat_1))
          (bind _output_get_4 (Variables|Default|SetGenerate_NoRepeat_2 _output_get_3))
          (Utilities|Array|Add (Variables|Default|GetGenerate_Return) _output_get_4)
          (else
            (goto _label))))
      (:2
        (bind _output_get_5 (Variables|Default|SetGenerate_Var (Math|Random|RandomIntegerinRange 1 17) :!label _label_2))
        (if (!= _output_get_5 (Variables|Default|GetGenerate_NoRepeat_1))
          (if (!= _output_get_5 (Variables|Default|GetGenerate_NoRepeat_2))
            (bind _output_get_6 (Variables|Default|SetGenerate_NoRepeat_2 _output_get_5))
            (Utilities|Array|Add (Variables|Default|GetGenerate_Return) _output_get_6)
            (else
              (goto _label_2)))
          (else
            (goto _label_2))))))
  (return (Variables|Default|GetGenerate_Return)))

(fn GetCardinTopic
  (params (Topic :type Array%20of%20Slate%20Brush%20Structures) (ID :type Integer))
  (bind _returnvalue (Math|Random|RandomIntegerinRange 0 3))
  (bind _returnvalue_2 (* ID 1e+02))
  (bind _cards_played (Variables|Default|GetCards_Played))
  (bind _returnvalue_3 (Math|Float|Truncate _returnvalue_2))
  (bind _returnvalue_4 (+ _returnvalue_3 _returnvalue))
  (Development|PrintString (Utilities|String|ToString(Integer) _returnvalue_4) true true "(R=1.000000,G=0.000000,B=0.099114,A=1.000000)" 5.0)
  (Utilities|FlowControl|Sequence :!label _label
    (:then_0
      (if (Utilities|Array|ContainsItem _cards_played _returnvalue_4)
        (goto _label)
        (else
          (Utilities|Array|Add _cards_played _returnvalue_4)
          (return (Utilities|Array|Get(acopy) Topic _returnvalue)))))))

(fn IDintoTopic
  (params (ID :type Integer)))